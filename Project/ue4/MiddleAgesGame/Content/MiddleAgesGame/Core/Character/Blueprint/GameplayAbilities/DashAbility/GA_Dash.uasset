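; Gameplay ability that makes the owning character dash forward.
; On activation it commits, zeroes the character's ground friction and applies a velocity-change impulse along the actor's forward vector while playing an assassin montage.
; When the montage completes, blends out, is interrupted or is cancelled, it restores the saved friction and ends the ability.
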(event Ability|EventActivateAbility
  (Ability|CommitAbility)
  (bind _ascharacter (Utilities|Casting|CastToCharacter (Ability|GetOwningActorfromActorInfo))
    (:then
      (Variables|Default|SetBaseGroundFriction (Variables|/Script/Engine.CharacterMovementComponent|GetGroundFriction (Variables|/Script/Engine.Character|GetCharacterMovement _ascharacter)))
      (Variables|/Script/Engine.CharacterMovementComponent|SetGroundFriction (Variables|/Script/Engine.Character|GetCharacterMovement _ascharacter) 0.0)
      (Physics|AddImpulse (Variables|/Script/Engine.Character|GetCharacterMovement _ascharacter) (* (Transformation|GetActorForwardVector _ascharacter) 2e+03) true)
      (|PlayMontageandWaitProxy "None" "/Game/MiddleAgesGame/Core/Character/Player/Animations/AM_Assassin_HealthAbility.AM_Assassin_HealthAbility" 1.0 "None" true 1.0
        (:OnCompleted
          _)
        (:OnBlendOut
          _)
        (:OnInterrupted
          _)
        (:OnCancelled
          _))
      (Variables|/Script/Engine.CharacterMovementComponent|SetGroundFriction (Variables|/Script/Engine.Character|GetCharacterMovement _ascharacter) (Variables|Default|GetBaseGroundFriction))
      (Ability|EndAbility))
    (:CastFailed
      (Ability|EndAbility))))