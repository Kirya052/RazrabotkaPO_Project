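; Spider enemy character built on the Gameplay Ability System, which acquires a melee ability on BeginPlay and triggers it through a MeleeAttack event.
; Capsule overlaps with a hostile player character send a deal-damage gameplay event to the spider itself, with the player as target.
; Health changes update its health bar widget, and Die plays a death montage before destroying the actor after a delay.
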(event OnComponentBeginOverlap(CapsuleCollider)
  (params (OverlappedComponent :type Primitive%20Component%20Object%20Reference) (OtherActor :type Actor%20Object%20Reference) (OtherComp :type Primitive%20Component%20Object%20Reference) (OtherBodyIndex :type Integer) (bFromSweep :type Boolean) (SweepResult :type Hit%20Result%20Structure%20%28by%20ref%29))
  (if (!= self OtherActor)
    (bind _asbp_player_character (Utilities|Casting|CastToBP_PlayerCharacter OtherActor))
    (bind _returnvalue (Class|AICharacter|IsOtherHostile self _asbp_player_character))
    (if _returnvalue
      (Ability|SendGameplayEventtoActor self "(TagName=\"skill.melee.dealDamage\")" (Utilities|Struct|MakeGameplayEventData "" 0 OtherActor))
      (Development|PrintString "damage player"))))

(event Custom|MeleeAttack
  (Abilities|TryActivateAbilitybyClass (Variables|Default|GetAbilitySystemComp) "/Game/MiddleAgesGame/Core/Character/Blueprint/GameplayAbilities/Melee/GA_Spider_Melee.GA_Spider_Melee_C" true)
  (Development|PrintString "Hello"))

(event EventBeginPlay
  (Class|AICharacter|AquireAbility "/Game/MiddleAgesGame/Core/Character/Blueprint/GameplayAbilities/Melee/GA_Spider_Melee.GA_Spider_Melee_C"))

(event EventDie
  (if (not (Variables|Default|GetbIsDead))
    (Animation|PlayAnimMontage "/Game/MiddleAgesGame/Core/Character/Blueprint/SpiderEnemy/Animation/AM_Spider_Death.AM_Spider_Death" 1.0 "None")
    (Utilities|FlowControl|Delay 3.0)
    (Actor|DestroyActor)))

(event EventOnHealthChanged
  (params (Health :type Float%20%28single-precision%29) (MaxHealth :type Float%20%28single-precision%29))
  (bind _aswb_health_bar (Utilities|Casting|CastToWB_HealthBar (UserInterface|GetUserWidgetObject (Variables|Default|GetHealthBar))))
  (Default|SetPercentage _aswb_health_bar (/ Health MaxHealth)))

(fn ConstructionScript)