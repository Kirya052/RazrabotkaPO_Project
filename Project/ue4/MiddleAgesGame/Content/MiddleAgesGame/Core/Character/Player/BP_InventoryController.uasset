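; BP_InventoryController is a player controller that handles inventory UI and melee attack input for the player character.
; OpenInventory toggles the WB_Inventory widget, creating it on first use, caching it and reusing it on later toggles.
; A custom event tells the cached widget to reload its inventory items.
; Attack casts the controlled pawn to BP_PlayerCharacter and calls its MeleeAttack.
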(event Custom|CustomEvent
  (bind _inventorywidget (Variables|Default|GetInventoryWidget))
  (Utilities|IsValid _inventorywidget
    (:Is%20Valid
      (Default|LoadInventoryItems (.AsWB%20Inventory (Utilities|Casting|CastToWB_Inventory _inventorywidget))))))

(event Input|ActionEvents|InputActionAttack
  (params (Key :type Key%20Structure :default "None"))
  ;[1 1 1] Melee Attack
  (:Pressed
    (bind _asbp_player_character (Utilities|Casting|CastToBP_PlayerCharacter (Pawn|GetControlledPawn)))
    (Default|MeleeAttack _asbp_player_character)))

(event Input|ActionEvents|InputActionOpenInventory
  (params (Key :type Key%20Structure :default "None"))
  (:Pressed
    ;[1 1 1] Toggle Inventory
    (Utilities|IsValid (Variables|Default|GetInventoryWidget)
      (:Is%20Valid
        (if (Widget|IsVisible (Variables|Default|GetInventoryWidget))
          (Widget|RemovefromParent (Variables|Default|GetInventoryWidget))
          (else
            (Utilities|IsValid (Variables|Default|GetInventoryWidget)
              (:Is%20Valid
                _)
              (:Is%20Not%20Valid
                (bind _returnvalue (UserInterface|CreateWidget "/Game/MiddleAgesGame/UI/Inventory/WB_Inventory.WB_Inventory_C" :!label _label))
                (bind _output_get (Variables|Default|SetInventoryWidget _returnvalue))))
            (UserInterface|Viewport|AddtoViewport (Variables|Default|GetInventoryWidget) 0))))
      (:Is%20Not%20Valid
        (goto _label)))))

(fn ConstructionScript)