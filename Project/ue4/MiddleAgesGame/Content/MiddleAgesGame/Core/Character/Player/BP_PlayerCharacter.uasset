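; Player character Blueprint that uses the Gameplay Ability System for melee attack, dash and health regen, granting all three abilities on BeginPlay.
; It creates a health bar widget and feeds it health, mana and stamina changes as ratios.
; Capsule overlaps with hostile assassin enemies send a deal-damage gameplay event to itself, targeting the enemy.
; A combo counter cycles three attack montages, and death plays a montage before destroying the actor.
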(event OnComponentBeginOverlap(CapsuleCollider)
  (params (OverlappedComponent :type Primitive%20Component%20Object%20Reference) (OtherActor :type Actor%20Object%20Reference) (OtherComp :type Primitive%20Component%20Object%20Reference) (OtherBodyIndex :type Integer) (bFromSweep :type Boolean) (SweepResult :type Hit%20Result%20Structure%20%28by%20ref%29))
  (if (!= self OtherActor)
    (bind _asbp_enemy_assasin (Utilities|Casting|CastToBP_EnemyAssasin OtherActor))
    (bind _returnvalue (Class|AICharacter|IsOtherHostile _asbp_enemy_assasin self))
    (if _returnvalue
      (Ability|SendGameplayEventtoActor self "(TagName=\"skill.melee.dealDamage\")" (Utilities|Struct|MakeGameplayEventData "" 0 OtherActor))
      (else
        (Development|PrintString "Hello")))))

(event Custom|MeleeAttack
  ;[1 1 1] Melee Attack
  (Abilities|TryActivateAbilitybyClass (Variables|Default|GetAbilitySystemComp) "/Game/MiddleAgesGame/Core/Character/Blueprint/GameplayAbilities/Melee/GA_Melee.GA_Melee_C" true))

(event Custom|TryHealthRegen
  ;[1 1 1] HealthRegen
  (Abilities|TryActivateAbilitybyClass (Variables|Default|GetAbilitySystemComp) "/Game/MiddleAgesGame/Core/Character/Blueprint/GameplayAbilities/HealthRegenAbility/GA_HealthRegen.GA_HealthRegen_C" true))

(event Custom|TryDashAbility
  (Abilities|TryActivateAbilitybyClass (Variables|Default|GetAbilitySystemComp) "/Game/MiddleAgesGame/Core/Character/Blueprint/GameplayAbilities/DashAbility/GA_Dash.GA_Dash_C" true))

(event Custom|EndCombo
  (Variables|Default|SetComboCount 0))

(event EventBeginPlay
  (Class|AssasinCharacter|AquireAbility "/Game/MiddleAgesGame/Core/Character/Blueprint/GameplayAbilities/Melee/GA_Melee.GA_Melee_C")
  (Class|AssasinCharacter|AquireAbility "/Game/MiddleAgesGame/Core/Character/Blueprint/GameplayAbilities/HealthRegenAbility/GA_HealthRegen.GA_HealthRegen_C")
  (Class|AssasinCharacter|AquireAbility "/Game/MiddleAgesGame/Core/Character/Blueprint/GameplayAbilities/DashAbility/GA_Dash.GA_Dash_C")
  (bind _returnvalue (UserInterface|CreateWidget "/Game/MiddleAgesGame/UI/PlayerStats/WB_PlayerHealthBar.WB_PlayerHealthBar_C"))
  (bind _output_get (Variables|Default|SetHealthBar _returnvalue))
  (UserInterface|Viewport|AddtoViewport _output_get 0))

(event EventOnManaChanged
  (params (Mana :type Float%20%28single-precision%29) (MaxMana :type Float%20%28single-precision%29))
  (Default|SetPercentageMana (Variables|Default|GetHealthBar) (/ Mana MaxMana)))

(event EventOnHealthChanged
  (params (Health :type Float%20%28single-precision%29) (MaxHealth :type Float%20%28single-precision%29))
  (Default|SetPercentageHealth (Variables|Default|GetHealthBar) (/ Health MaxHealth)))

(event EventDIe
  (if (not (Variables|Default|GetbIsDead))
    (Animation|PlayAnimMontage "/Game/MiddleAgesGame/Core/Character/Player/Animations/AM_AssasinDead.AM_AssasinDead" 1.0 "None")
    (Utilities|FlowControl|Delay 3.0)
    (Actor|DestroyActor)))

(event EventOnStaminaChanged
  (params (Stamina :type Float%20%28single-precision%29) (MaxStamina :type Float%20%28single-precision%29))
  (Default|SetPercentageStamina (Variables|Default|GetHealthBar) (/ Stamina MaxStamina)))

(fn ConstructionScript)

(fn DeterminCombo
  (switch int (Variables|Default|GetComboCount)
    (:0
      (Variables|Default|SetAnimMontageCombo "/Game/MiddleAgesGame/Core/Character/Player/Animations/AM_MeleeBase.AM_MeleeBase")
      (Math|Integer|IncrementInt (Variables|Default|GetComboCount) :!label _label))
    (:1
      (Variables|Default|SetAnimMontageCombo "/Game/MiddleAgesGame/Core/Character/Player/Animations/AM_MeleeAttack4.AM_MeleeAttack4")
      (goto _label))
    (:2
      (Variables|Default|SetAnimMontageCombo "/Game/MiddleAgesGame/Core/Character/Player/Animations/AM_MeleeAttack3.AM_MeleeAttack3")
      (Variables|Default|SetComboCount 0))))