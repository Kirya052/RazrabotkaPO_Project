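; BP_RunTest is a functional test that checks a referenced Character can crouch, jump and run forward into a trigger.
; StartTest runs a delayed sequence of crouch, uncrouch and jump, then sets StartRun.
; While StartRun is set, Tick feeds forward movement input to the Character.
; Any actor beginning overlap with Trigger finishes the test as Succeeded, with no check on crouch or jump results.
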(event OnActorBeginOverlap(Trigger)
  (params (OverlappedActor :type Actor%20Object%20Reference) (OtherActor :type Actor%20Object%20Reference))
  (Class|FunctionalTest|FinishTest "Succeeded"))

(event EventStartTest
  (bind _character (Variables|Default|GetCharacter))
  (Variables|Default|SetStartRun false)
  (Character|Crouch _character)
  (Utilities|FlowControl|Delay 0.5)
  (Character|UnCrouch _character)
  (Utilities|FlowControl|Delay 0.5)
  (Character|Jump _character)
  (Utilities|FlowControl|Delay 1.0)
  (Variables|Default|SetStartRun true))

(event EventTick
  (params (DeltaSeconds :type Float%20%28single-precision%29))
  (bind _character (Variables|Default|GetCharacter))
  (if (Variables|Default|GetStartRun)
    (Pawn|Input|AddMovementInput _character (Transformation|GetActorForwardVector _character) 1.0 false)))

(fn ConstructionScript)